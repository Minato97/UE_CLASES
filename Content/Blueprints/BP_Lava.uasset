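; BP_Lava is a lava hazard actor that moves vertically and can kill the player.
; On BeginPlay it stores its starting position, then the ActualizarAltura timeline lerps its Z toward that height plus Altura.
; OnCollisionDetecter prints a death message and, if Destruir is set, destroys the passed Jugador, plays an 8-bit death sound, shows the BP_Wid_Muerto widget and enables the mouse cursor.
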(event `self.ReceiveBeginPlay`
  (bind (_pos_initial_x _pos_initial_y _pos_initial_z) (`KismetMathLibrary.BreakVector` (`self.Pos_Initial`)))
  (set `self.Pos_Initial` (`SceneComponent.K2_GetComponentLocation` (`self.DefaultSceneRoot`)))
  (bind (_direction _pista_nueva_1) (`Timeline|ActualizarAltura`)
    (:`Update`
      (`self.K2_SetActorLocation` (`KismetMathLibrary.MakeVector` _pos_initial_x _pos_initial_y (`KismetMathLibrary.Lerp` _pos_initial_z (+ _pos_initial_z (`self.Altura`)) _pista_nueva_1))))))

(event `/Game/Blueprints/BPI_ColisionDetecter.onCollisionDetecter`
  (params (jugador :type "/Game/ThirdPerson/Blueprints/BP_ThirdPersonCharacter Object Reference"))
  (`KismetSystemLibrary.PrintString` "Estas Morido!")
  (if (`self.Destruir`)
    (`self.K2_DestroyActor` jugador)
    (`GameplayStatics.PlaySoundAtLocation` "/Game/sonidos/dead-8bit-41400.dead-8bit-41400" (`self.K2_GetActorLocation`) (struct) 1.0 1.0 0.0 null null null null)
    (bind _returnvalue (`|CreateWidget` "/Game/Blueprints/BP_Wid_Muerto.BP_Wid_Muerto_C"))
    (`UserWidget.AddToViewport` _returnvalue 0)
    (set `PlayerController.bShowMouseCursor` true (`GameplayStatics.GetPlayerController` 0))))

(fn `UserConstructionScript`)